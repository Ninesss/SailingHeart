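; BP_SHGridBase is a base grid Blueprint that drives the visual border around its placeable area.
; InitializeBorder forwards height, corner and style settings to the BP_Mesh_Border and BP_Decal_Border actors.
; UpdateBorderSize resizes both borders to the grid's placeable width and height.
; Each border is cast on its own Sequence branch, so a missing mesh or decal actor does not block the other.
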(event `self.UpdateBorderSize`
  (`|ExecutionSequence`
    (:`then_0`
      (bind _asbp_mesh_border (cast `/Game/MapBorderCollection/Blueprints/BP_Mesh_Border` (`self.MeshBorderActor`)))
      (`/Game/MapBorderCollection/Blueprints/BP_Mesh_Border.UpdateBorderSize` _asbp_mesh_border (`self.GetPlaceableWidth`) (`self.GetPlaceableHeight`)))
    (:`then_1`
      (bind _asbp_decal_border (cast `/Game/MapBorderCollection/Blueprints/BP_Decal_Border` (`self.DecalBorderActor`)))
      (`/Game/MapBorderCollection/Blueprints/BP_Decal_Border.UpdateBorderSize` _asbp_decal_border (`self.GetPlaceableWidth`) (`self.GetPlaceableHeight`)))))

(event `self.InitializeBorder`
  (`|ExecutionSequence`
    (:`then_0`
      (bind _asbp_mesh_border (cast `/Game/MapBorderCollection/Blueprints/BP_Mesh_Border` (`self.MeshBorderActor`)))
      (`/Game/MapBorderCollection/Blueprints/BP_Mesh_Border.InitializeBorder` _asbp_mesh_border (`self.BorderHeight`) (`self.CornerRoundness`) (`self.BorderMaterial`)))
    (:`then_1`
      (bind _asbp_decal_border (cast `/Game/MapBorderCollection/Blueprints/BP_Decal_Border` (`self.DecalBorderActor`)))
      (`/Game/MapBorderCollection/Blueprints/BP_Decal_Border.InitializeBorder` _asbp_decal_border (`self.BorderHeight`) (`self.BorderLineThickness`) (`self.CornerRoundness`) (`self.DecalBorderColor`) (`self.BorderSharpness`)))))

(fn `UserConstructionScript`)