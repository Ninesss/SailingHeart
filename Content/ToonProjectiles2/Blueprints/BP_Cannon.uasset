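; BP_Cannon is a cursor-aimed cannon that fires any of fifteen toon projectile Blueprints, apparently for showcasing the effects.
; Each tick, it turns its Sphere toward the world-static hit under the cursor.
; Left click spawns the selected projectile at FirePoint with the Sphere's rotation, while holding right click repeats this through a short Delay.
; A/D or Left/Right keys cycle the selection with wraparound.
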(event `Key|Right`
  (params (Key :type "Key Structure"))
  (bind _returnvalue (+ 1.0 (`self.Effect Number`)))
  (:`Pressed`
    (if (> _returnvalue (- (`KismetMathLibrary.Conv_IntToDouble` (`KismetArrayLibrary.Array_Length` (`|MakeArray` "/Game/ToonProjectiles2/Blueprints/BP_Projectile_1.BP_Projectile_1_C" "/Game/ToonProjectiles2/Blueprints/BP_Projectile_2.BP_Projectile_2_C" "/Game/ToonProjectiles2/Blueprints/BP_Projectile_3.BP_Projectile_3_C" "/Game/ToonProjectiles2/Blueprints/BP_Projectile_4.BP_Projectile_4_C" "/Game/ToonProjectiles2/Blueprints/BP_Projectile_5.BP_Projectile_5_C" "/Game/ToonProjectiles2/Blueprints/BP_Projectile_6.BP_Projectile_6_C" "/Game/ToonProjectiles2/Blueprints/BP_Projectile_7.BP_Projectile_7_C" "/Game/ToonProjectiles2/Blueprints/BP_Projectile_8.BP_Projectile_8_C" "/Game/ToonProjectiles2/Blueprints/BP_Projectile_9.BP_Projectile_9_C" "/Game/ToonProjectiles2/Blueprints/BP_Projectile_10.BP_Projectile_10_C" "/Game/ToonProjectiles2/Blueprints/BP_Projectile_11.BP_Projectile_11_C" "/Game/ToonProjectiles2/Blueprints/BP_Projectile_12.BP_Projectile_12_C" "/Game/ToonProjectiles2/Blueprints/BP_Projectile_13.BP_Projectile_13_C" "/Game/ToonProjectiles2/Blueprints/BP_Projectile_14.BP_Projectile_14_C" "/Game/ToonProjectiles2/Blueprints/BP_Projectile_15.BP_Projectile_15_C" :!type "Actor Class Reference"))) 1.0)) :!label _label
      (set `self.Effect Number` 0.0)
      (else
        (set `self.Effect Number` _returnvalue)))))

(event `Key|D`
  (params (Key :type "Key Structure"))
  (:`Pressed`
    (goto _label)))

(event `Key|Left`
  (params (Key :type "Key Structure"))
  (bind _returnvalue (- (`self.Effect Number`) 1.0))
  (:`Pressed`
    (if (> 0.0 _returnvalue) :!label _label_2
      (set `self.Effect Number` (- (`KismetMathLibrary.Conv_IntToDouble` (`KismetArrayLibrary.Array_Length` (`|MakeArray` "/Game/ToonProjectiles2/Blueprints/BP_Projectile_1.BP_Projectile_1_C" "/Game/ToonProjectiles2/Blueprints/BP_Projectile_2.BP_Projectile_2_C" "/Game/ToonProjectiles2/Blueprints/BP_Projectile_3.BP_Projectile_3_C" "/Game/ToonProjectiles2/Blueprints/BP_Projectile_4.BP_Projectile_4_C" "/Game/ToonProjectiles2/Blueprints/BP_Projectile_5.BP_Projectile_5_C" "/Game/ToonProjectiles2/Blueprints/BP_Projectile_6.BP_Projectile_6_C" "/Game/ToonProjectiles2/Blueprints/BP_Projectile_7.BP_Projectile_7_C" "/Game/ToonProjectiles2/Blueprints/BP_Projectile_8.BP_Projectile_8_C" "/Game/ToonProjectiles2/Blueprints/BP_Projectile_9.BP_Projectile_9_C" "/Game/ToonProjectiles2/Blueprints/BP_Projectile_10.BP_Projectile_10_C" "/Game/ToonProjectiles2/Blueprints/BP_Projectile_11.BP_Projectile_11_C" "/Game/ToonProjectiles2/Blueprints/BP_Projectile_12.BP_Projectile_12_C" "/Game/ToonProjectiles2/Blueprints/BP_Projectile_13.BP_Projectile_13_C" "/Game/ToonProjectiles2/Blueprints/BP_Projectile_14.BP_Projectile_14_C" "/Game/ToonProjectiles2/Blueprints/BP_Projectile_15.BP_Projectile_15_C" :!type "Actor Class Reference"))) 1.0))
      (else
        (set `self.Effect Number` _returnvalue)))))

(event `Key|A`
  (params (Key :type "Key Structure"))
  (:`Pressed`
    (goto _label_2)))

(event `Key|LeftMouseButton`
  (params (Key :type "Key Structure"))
  (:`Pressed`
    (`|SpawnActorFromClass` (`|GetArrayItem` (`|MakeArray` "/Game/ToonProjectiles2/Blueprints/BP_Projectile_1.BP_Projectile_1_C" "/Game/ToonProjectiles2/Blueprints/BP_Projectile_2.BP_Projectile_2_C" "/Game/ToonProjectiles2/Blueprints/BP_Projectile_3.BP_Projectile_3_C" "/Game/ToonProjectiles2/Blueprints/BP_Projectile_4.BP_Projectile_4_C" "/Game/ToonProjectiles2/Blueprints/BP_Projectile_5.BP_Projectile_5_C" "/Game/ToonProjectiles2/Blueprints/BP_Projectile_6.BP_Projectile_6_C" "/Game/ToonProjectiles2/Blueprints/BP_Projectile_7.BP_Projectile_7_C" "/Game/ToonProjectiles2/Blueprints/BP_Projectile_8.BP_Projectile_8_C" "/Game/ToonProjectiles2/Blueprints/BP_Projectile_9.BP_Projectile_9_C" "/Game/ToonProjectiles2/Blueprints/BP_Projectile_10.BP_Projectile_10_C" "/Game/ToonProjectiles2/Blueprints/BP_Projectile_11.BP_Projectile_11_C" "/Game/ToonProjectiles2/Blueprints/BP_Projectile_12.BP_Projectile_12_C" "/Game/ToonProjectiles2/Blueprints/BP_Projectile_13.BP_Projectile_13_C" "/Game/ToonProjectiles2/Blueprints/BP_Projectile_14.BP_Projectile_14_C" "/Game/ToonProjectiles2/Blueprints/BP_Projectile_15.BP_Projectile_15_C" :!type "Actor Class Reference") (`KismetMathLibrary.FTrunc` (`self.Effect Number`))) (`KismetMathLibrary.MakeTransform` (`SceneComponent.K2_GetComponentLocation` (`self.FirePoint`)) (`SceneComponent.K2_GetComponentRotation` (`self.Sphere`))) "Undefined" "OverrideRootScale" null null :!label _label_3)))

(event `self.ReceiveTick`
  (params (DeltaSeconds :type "Float (single-precision)"))
  (bind _returnvalue (`GameplayStatics.GetPlayerController` 0))
  (`SceneComponent.K2_SetWorldRotation` (`self.Sphere`) (`KismetMathLibrary.FindLookAtRotation` (`SceneComponent.K2_GetComponentLocation` (`self.FirePoint`)) (`.Location` (`GameplayStatics.BreakHitResult` (`PlayerController.GetHitResultUnderCursorForObjects` _returnvalue (`|MakeArray` "ObjectTypeQuery1" :!type "EObjectTypeQuery Enum") true)))) false false)
  (if (`PlayerController.IsInputKeyDown` _returnvalue "RightMouseButton")
    (`KismetSystemLibrary.Delay` 0.1)
    (goto _label_3)))

(fn `UserConstructionScript`)